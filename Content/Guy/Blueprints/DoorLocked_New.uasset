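; DoorLocked_New is a locked door whose Glass panel slides vertically once its Open flag is set.
; Tick watches Open and spawns a one-time particle effect above the Frame.
; Box overlap with the runner character opens a gate on Interact input, which FlipFlops between open and close timelines lerping the Glass height.
; DoneOpen, set after a delay in each timeline update, guards against reversing too early.
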(event OnComponentBeginOverlap(Box)
  (params (OverlappedComponent :type Primitive%20Component%20Object%20Reference) (OtherActor :type Actor%20Object%20Reference) (OtherComp :type Primitive%20Component%20Object%20Reference) (OtherBodyIndex :type Integer) (bFromSweep :type Boolean) (SweepResult :type Hit%20Result%20Structure%20%28by%20ref%29))
  (bind _glass (Variables|Default|GetGlass))
  (bind _glass_2 (Variables|Default|GetGlass))
  (bind _relativelocation (Variables|/Script/Engine.SceneComponent|GetRelativeLocation _glass))
  (bind _relativelocation_2 (Variables|/Script/Engine.SceneComponent|GetRelativeLocation _glass_2))
  ;[1 1 1] Interact
  (Utilities|Casting|CastToCharacter_RunnerBP_SideKnifes OtherActor)
  (Utilities|FlowControl|Gate true) ; enters at Open
)

(event OnComponentEndOverlap(Box)
  (params (OverlappedComponent :type Primitive%20Component%20Object%20Reference) (OtherActor :type Actor%20Object%20Reference) (OtherComp :type Primitive%20Component%20Object%20Reference) (OtherBodyIndex :type Integer))
  (bind _glass (Variables|Default|GetGlass))
  (bind _glass_2 (Variables|Default|GetGlass))
  (bind _relativelocation (Variables|/Script/Engine.SceneComponent|GetRelativeLocation _glass))
  (bind _relativelocation_2 (Variables|/Script/Engine.SceneComponent|GetRelativeLocation _glass_2))
  ;[1 1 1] Interact
  (Utilities|Casting|CastToCharacter_RunnerBP_SideKnifes OtherActor)
  (Utilities|FlowControl|Gate true) ; enters at Close
)

(event Collision|EventActorBeginOverlap
  (params (OtherActor :type Actor%20Object%20Reference)))

(event EventTick
  (params (DeltaSeconds :type Float%20%28single-precision%29))
  (if (Variables|Default|GetOpen?)
    (Utilities|FlowControl|DoOnce false
      (:Completed
        (Effects|SpawnEmitteratLocation "/Game/Guy/ParticleSystem/DoorLocked_Effect.DoorLocked_Effect" (+ (Transformation|GetWorldLocation (Variables|Default|GetFrame)) "0,0,300.000000"))))))

(event EventBeginPlay
  ;[1 1 1] Enable Input
  (Input|EnableInput (Game|GetPlayerController 0)))

(event Input|ActionEvents|InputActionInteract
  (params (Key :type Key%20Structure :default "None"))
  (bind _glass (Variables|Default|GetGlass))
  (bind _glass_2 (Variables|Default|GetGlass))
  (bind _relativelocation (Variables|/Script/Engine.SceneComponent|GetRelativeLocation _glass))
  (bind _relativelocation_2 (Variables|/Script/Engine.SceneComponent|GetRelativeLocation _glass_2))
  ;[1 1 1] Interact
  (:Pressed
    (if (Variables|Default|GetOpen?)
      (Utilities|FlowControl|Gate true
        (:Exit
          (Utilities|FlowControl|FlipFlop
            (:A
              (if (not (Variables|Default|GetDoneOpen?))
                ;[1 1 1] Door Open
                (Utilities|FlowControl|Sequence
                  (:then_0
                    (bind _leftdooropen (Timeline|Timeline_0 PlayFromStart)
                      (:Update
                        (Transformation|SetRelativeLocation _glass_2 (Math|Vector|MakeVector (.x _relativelocation_2) (.y _relativelocation_2) (Math|Float|Lerp (Variables|Default|GetLeft_Door_Close_Float) (Variables|Default|GetLeft_Door_Open_Float) _leftdooropen)) false false)
                        (Utilities|FlowControl|Delay 3.0)
                        (Variables|Default|SetDoneOpen? true)))))))
            (:B
              (if (Variables|Default|GetDoneOpen?)
                ;[1 1 1] Door Close
                (Utilities|FlowControl|Sequence
                  (:then_0
                    (bind _leftdooropen_2 (Timeline|Timeline_2 ReverseFromEnd)
                      (:Update
                        (Transformation|SetRelativeLocation _glass (Math|Vector|MakeVector (.x _relativelocation) (.y _relativelocation) (Math|Float|Lerp (Variables|Default|GetLeft_Door_Close_Float) (Variables|Default|GetLeft_Door_Open_Float) _leftdooropen_2)) false false)
                        (Utilities|FlowControl|Delay 3.0)
                        (Variables|Default|SetDoneOpen? false)))))))))))))

(fn ConstructionScript)