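; Alien enemy AI character with sound, filed as not in use, that wanders randomly and chases and bashes the player on sight.
; Pawn sensing sets run speed and CanSee, which a retriggerable delay clears; successful attacks subtract from Maze_GameMode health.
; A DoOnce starts the chase sound, and Tick fades it out and resets once sight is lost.
; Capsule overlap with an attacking player damages it, playing hit or random death animations before destruction.
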(event OnComponentBeginOverlap(CapsuleComponent)
  (params (OverlappedComponent :type Primitive%20Component%20Object%20Reference) (OtherActor :type Actor%20Object%20Reference) (OtherComp :type Primitive%20Component%20Object%20Reference) (OtherBodyIndex :type Integer) (bFromSweep :type Boolean) (SweepResult :type Hit%20Result%20Structure%20%28by%20ref%29))
  (bind _charactermovement (Variables|Character|GetCharacterMovement))
  ;[1 1 1] Taking Damage
  (bind _ascharacter_runner_bp_side_knifes (Utilities|Casting|CastToCharacter_RunnerBP_SideKnifes OtherActor))
  (if (Variables|/Game/Guy/Blueprints/Character_RunnerBP_SideKnifes.Character_RunnerBP_SideKnifes_C|GetAttacking? _ascharacter_runner_bp_side_knifes)
    (if (not (Variables|Default|GetGetDamage?))
      (Variables|Default|SetGetDamage? true)
      (bind _output_get (Variables|Default|SetHealth (- (Variables|Default|GetHealth) (Variables|Default|GetDamage))))
      (Development|PrintString (Utilities|String|ToString(Float) _output_get))
      (Components|Movement|StopMovementImmediately _charactermovement)
      (Pawn|Components|CharacterMovement|DisableMovement _charactermovement)
      (if (> (Variables|Default|GetHealth) 0.1)
        ;;[1 1 1] Still Alive
        (Components|Animation|PlayAnimation (Variables|Character|GetMesh) "/Game/Guy/Character_AlienEnemy/Animations/Head_Hit.Head_Hit" false)
        (Utilities|FlowControl|Delay 1.3)
        (Variables|Default|SetGetDamage? false)
        (Components|Animation|SetAnimationMode (Variables|Character|GetMesh) "AnimationBlueprint") ; ?Returning the AnimBP
        (Pawn|Components|CharacterMovement|SetMovementMode (Variables|Character|GetCharacterMovement) "MOVE_Walking" 0)
        (else
          ;;[1 1 1] Death
          (Variables|Default|SetDead? true)
          (switch int (Math|Random|RandomIntegerinRange 0 3)
            (:Default
              (Components|Animation|PlayAnimation (Variables|Character|GetMesh) "/Game/Guy/Character_AlienEnemy/Animations/Death_From_Back_Headshot.Death_From_Back_Headshot" false :!label _label))
            (:0
              (goto _label))
            (:1
              (Components|Animation|PlayAnimation (Variables|Character|GetMesh) "/Game/Guy/Character_AlienEnemy/Animations/Death_From_Front_Headshot.Death_From_Front_Headshot" false))
            (:2
              (Components|Animation|PlayAnimation (Variables|Character|GetMesh) "/Game/Guy/Character_AlienEnemy/Animations/Falling_Back_Death.Falling_Back_Death" false))
            (:3
              (Components|Animation|PlayAnimation (Variables|Character|GetMesh) "/Game/Guy/Character_AlienEnemy/Animations/Falling_Forward_Death.Falling_Forward_Death" false)))
          (Utilities|FlowControl|Delay 12.0)
          (Actor|DestroyActor)
          (Audio|Components|Audio|FadeOut (Variables|Default|GetEnemySound) 0.1 0.0 "Linear" :!class /Script/Engine.AudioComponent))))))

(event OnSeePawn(PawnSensing(Eyes))
  (params (Pawn :type Pawn%20Object%20Reference))
  (bind _mesh (Variables|Character|GetMesh))
  ;[1 1 1] AI Chase Player & Sound
  ;;[1 1 1] Eyes - Chase Player
  (if (not (Variables|Default|GetDead?))
    (bind _ascharacter_runner_bp_side_knifes (Utilities|Casting|CastToCharacter_RunnerBP_SideKnifes Pawn))
    (Utilities|FlowControl|Sequence
      (:then_0
        (Variables|Default|SetCanSee? true)
        (Variables|/Script/Engine.CharacterMovementComponent|SetMaxWalkSpeed (Variables|Character|GetCharacterMovement) (Variables|Default|GetMAX_RUN))
        (AI|AIMoveTo self "0, 0, 0" _ascharacter_runner_bp_side_knifes 5.0 false
          (:then
            ;;;[0 0.3557 1] Play Sound
            (Utilities|FlowControl|DoOnce false ; Reset should be connected to fade out sound
              (:Completed
                (Audio|Components|Audio|Play (Variables|Default|GetEnemySound) 0.0))))
          (:OnSuccess
            ;;;[1 0 0.0169] Attack
            (Utilities|FlowControl|Delay 0.3)
            (if (not (Variables|Default|GetGetDamage?)) ; Disconnect it if want to be able attack when getting damage
              (if (not (Variables|Default|GetDead?))
                (Components|Animation|PlayAnimation _mesh "/Game/Guy/Character_AlienEnemy/Animations/Bash.Bash" false)
                (Utilities|FlowControl|Delay 1.0)
                (Components|Animation|SetAnimationMode _mesh "AnimationBlueprint")
                (if (Variables|Default|GetCanSee?)
                  (bind _asmaze_game_mode (Utilities|Casting|CastToMaze_GameMode (Game|GetGameMode)))
                  (Variables|/Game/Guy/Blueprints/Maze_GameMode.Maze_GameMode_C|SetHealth _asmaze_game_mode (- (Variables|/Game/Guy/Blueprints/Maze_GameMode.Maze_GameMode_C|GetHealth _asmaze_game_mode) (Variables|Default|GetDamage)))))))))
      (:then_1
        ;;;[1 1 1] Hide eyes
        (Utilities|FlowControl|RetriggerableDelay 0.6)
        (Variables|/Script/Engine.CharacterMovementComponent|SetMaxWalkSpeed (Variables|Character|GetCharacterMovement) (Variables|Default|GetMAX_WALK))
        (Variables|Default|SetCanSee? false)))))

(event EventBeginPlay
  ;[1 1 1] AI Chase Player & Sound
  ;;[1 1 1] Load Sound
  (bind _returnvalue (AddComponent|AddAudioComponent false))
  (Audio|Components|Audio|Stop _returnvalue)
  (Variables|Default|SetEnemySound _returnvalue))

(event Collision|EventActorBeginOverlap
  (params (OtherActor :type Actor%20Object%20Reference)))

(event EventTick
  (params (DeltaSeconds :type Float%20%28single-precision%29))
  (Utilities|FlowControl|Sequence
    (:then_0
      ;[1 1 1] Walk
      (if (not (Variables|Default|GetDead?))
        (if (not (Variables|Default|GetCanSee?))
          (if (not (Variables|Default|GetGetDamage?))
            (Utilities|FlowControl|Delay (Math|Random|RandomFloatinRange 1.0 5.0))
            (AI|AIMoveTo self (.RandomLocation (AI|Navigation|GetRandomReachablePointinRadius (Transformation|GetActorLocation) 1.5e+03 0 0)) 0 5.0 true)))))
    (:then_1
      ;[1 1 1] AI Chase Player & Sound
      ;;[1 1 1] Event Tick - Fade out sound
      (if (not (Variables|Default|GetCanSee?))
        (Utilities|FlowControl|Delay 0.4)
        (if (not (Variables|Default|GetCanSee?))
          (Audio|Components|Audio|FadeOut (Variables|Default|GetEnemySound) 0.3 0.0 "Linear" :!class /Script/Engine.AudioComponent) ; After fade out - reset the play option
          ;;[1 1 1] Eyes - Chase Player
          ;;;[0 0.3557 1] Play Sound
          (Utilities|FlowControl|DoOnce false) ; enters at Reset
        )))))

(fn ConstructionScript)