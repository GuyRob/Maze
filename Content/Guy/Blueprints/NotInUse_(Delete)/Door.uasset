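; Sliding glass door that opens when the player's runner character enters its Box trigger and closes when they leave.
; Separate opening and closing timelines nudge Glass along local Y by adding scaled track values each update, so movement accumulates rather than interpolating between fixed positions.
; Two DoOnce gates, re-armed after short delays by the opposite overlap event, limit retriggering; debug prints remain marked for deletion.
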(event OnComponentBeginOverlap(Box)
  (params (OverlappedComponent :type Primitive%20Component%20Object%20Reference) (OtherActor :type Actor%20Object%20Reference) (OtherComp :type Primitive%20Component%20Object%20Reference) (OtherBodyIndex :type Integer) (bFromSweep :type Boolean) (SweepResult :type Hit%20Result%20Structure%20%28by%20ref%29))
  (bind _glass (Variables|Default|GetGlass))
  (bind _glass_2 (Variables|Default|GetGlass))
  (bind _ascharacter_runner_bp_side_knifes (Utilities|Casting|CastToCharacter_RunnerBP_SideKnifes (Game|GetPlayerCharacter 0)))
  (if (== OtherActor _ascharacter_runner_bp_side_knifes)
    (Utilities|FlowControl|Sequence
      (:then_0
        (Utilities|FlowControl|Delay 0.2)
        (Utilities|FlowControl|DoOnce false) ; enters at Reset
      )
      (:then_1
        (Utilities|FlowControl|DoOnce false
          (:Completed
            (Development|PrintString "Hello") ; DELETE
            (bind _newtrack_0 (Timeline|Open%20Door PlayFromStart)
              (:Update
                (Transformation|SetRelativeLocation _glass_2 (+ (Variables|/Script/Engine.SceneComponent|GetRelativeLocation _glass_2) (Math|Vector|MakeVector 0.0 (* _newtrack_0 -1e+01) 0.0)) false false)))))))))

(event OnComponentEndOverlap(Box)
  (params (OverlappedComponent :type Primitive%20Component%20Object%20Reference) (OtherActor :type Actor%20Object%20Reference) (OtherComp :type Primitive%20Component%20Object%20Reference) (OtherBodyIndex :type Integer))
  (bind _glass (Variables|Default|GetGlass))
  (bind _glass_2 (Variables|Default|GetGlass))
  (bind _ascharacter_runner_bp_side_knifes (Utilities|Casting|CastToCharacter_RunnerBP_SideKnifes (Game|GetPlayerCharacter 0)))
  (if (== OtherActor _ascharacter_runner_bp_side_knifes)
    (Utilities|FlowControl|Sequence
      (:then_0
        (Utilities|FlowControl|Delay 1.0)
        (Utilities|FlowControl|DoOnce false) ; enters at Reset
      )
      (:then_1
        (Utilities|FlowControl|DoOnce false
          (:Completed
            (Development|PrintString "Bye") ; DELETE
            (bind _newtrack_0 (Timeline|Timeline_0 ReverseFromEnd)
              (:Update
                (Transformation|SetRelativeLocation _glass (+ (Variables|/Script/Engine.SceneComponent|GetRelativeLocation _glass) (Math|Vector|MakeVector 0.0 (* _newtrack_0 1e+01) 0.0)) false false)))))))))

(event EventBeginPlay)

(event Collision|EventActorBeginOverlap
  (params (OtherActor :type Actor%20Object%20Reference)))

(event EventTick
  (params (DeltaSeconds :type Float%20%28single-precision%29)))

(fn ConstructionScript)