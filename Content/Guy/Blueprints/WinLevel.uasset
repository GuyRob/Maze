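; WinLevel is a level-end trigger actor that finishes the current maze level when the Character_RunnerBP_SideKnifes player overlaps its Box.
; While Maze_GameMode's Level is below MAXLEVEL, a DoOnce shows FinishLevel_Widget, waits briefly, increments Level and destroys the character.
; Otherwise it creates FinishGame_Widget without adding it to the viewport and prints that no levels remain.
; The character leaving the Box resets the DoOnce.
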(event OnComponentEndOverlap(Box)
  (params (OverlappedComponent :type Primitive%20Component%20Object%20Reference) (OtherActor :type Actor%20Object%20Reference) (OtherComp :type Primitive%20Component%20Object%20Reference) (OtherBodyIndex :type Integer))
  (Utilities|Casting|CastToCharacter_RunnerBP_SideKnifes OtherActor)
  (Utilities|FlowControl|DoOnce false ; enters at Reset
    (:Completed
      (UserInterface|CreateWidget "/Game/Guy/Blueprints/FinishGame_Widget.FinishGame_Widget_C")
      (Development|PrintString "No More Levels!" true true "(R=0.000000,G=1.000000,B=0.024297,A=1.000000)"))))

(event OnComponentBeginOverlap(Box)
  (params (OverlappedComponent :type Primitive%20Component%20Object%20Reference) (OtherActor :type Actor%20Object%20Reference) (OtherComp :type Primitive%20Component%20Object%20Reference) (OtherBodyIndex :type Integer) (bFromSweep :type Boolean) (SweepResult :type Hit%20Result%20Structure%20%28by%20ref%29))
  (bind _ascharacter_runner_bp_side_knifes (Utilities|Casting|CastToCharacter_RunnerBP_SideKnifes OtherActor))
  (if (Variables|/Game/Guy/Blueprints/Character_RunnerBP_SideKnifes.Character_RunnerBP_SideKnifes_C|GetInteract? _ascharacter_runner_bp_side_knifes)
    _
    (else
      _))
  (bind _asmaze_game_mode (Utilities|Casting|CastToMaze_GameMode (Game|GetGameMode)))
  (if (< (Variables|/Game/Guy/Blueprints/Maze_GameMode.Maze_GameMode_C|GetLevel _asmaze_game_mode) (Variables|/Game/Guy/Blueprints/Maze_GameMode.Maze_GameMode_C|GetMAX_LEVEL _asmaze_game_mode))
    (Utilities|FlowControl|DoOnce false
      (:Completed
        (bind _returnvalue (UserInterface|CreateWidget "/Game/Guy/Blueprints/FinishLevel_Widget.FinishLevel_Widget_C"))
        (UserInterface|Viewport|AddtoViewport _returnvalue 0)
        (Utilities|FlowControl|Delay 2.5)
        (Variables|/Game/Guy/Blueprints/Maze_GameMode.Maze_GameMode_C|SetLevel _asmaze_game_mode (+ (Variables|/Game/Guy/Blueprints/Maze_GameMode.Maze_GameMode_C|GetLevel _asmaze_game_mode) 1))
        (Actor|DestroyActor _ascharacter_runner_bp_side_knifes)))
    (else
      (UserInterface|CreateWidget "/Game/Guy/Blueprints/FinishGame_Widget.FinishGame_Widget_C")
      (Development|PrintString "No More Levels!" true true "(R=0.000000,G=1.000000,B=0.024297,A=1.000000)"))))

(event EventBeginPlay)

(event Collision|EventActorBeginOverlap
  (params (OtherActor :type Actor%20Object%20Reference)))

(event EventTick
  (params (DeltaSeconds :type Float%20%28single-precision%29)))

(fn ConstructionScript)