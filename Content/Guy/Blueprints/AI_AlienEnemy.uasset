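; AI alien enemy character that wanders, chases the player's runner and trades melee hits with it.
; Tick drives random roaming; pawn sensing triggers a faster chase, with a retriggerable delay clearing sight.
; Reaching the runner plays a bash that lowers GameMode health (block-aware) and handles player death UI.
; Capsule overlap with an attacking runner damages the alien; hit and death animations temporarily override the AnimBP, and enemy sound is disconnected.
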(event OnComponentBeginOverlap(CapsuleComponent)
  (params (OverlappedComponent :type Primitive%20Component%20Object%20Reference) (OtherActor :type Actor%20Object%20Reference) (OtherComp :type Primitive%20Component%20Object%20Reference) (OtherBodyIndex :type Integer) (bFromSweep :type Boolean) (SweepResult :type Hit%20Result%20Structure%20%28by%20ref%29))
  (bind _charactermovement (Variables|Character|GetCharacterMovement))
  ;[1 1 1] Taking Damage
  (bind _ascharacter_runner_bp_side_knifes (Utilities|Casting|CastToCharacter_RunnerBP_SideKnifes OtherActor))
  (if (Variables|/Game/Guy/Blueprints/Character_RunnerBP_SideKnifes.Character_RunnerBP_SideKnifes_C|GetAttacking? _ascharacter_runner_bp_side_knifes)
    (if (not (Variables|Default|GetGetDamage?))
      (Variables|Default|SetGetDamage? true)
      (bind _output_get (Variables|Default|SetHealth (- (Variables|Default|GetHealth) (Variables|Default|GetZombieTakeDamage))))
      (Development|PrintString (Utilities|String|ToString(Float) _output_get))
      (Components|Movement|StopMovementImmediately _charactermovement)
      (Pawn|Components|CharacterMovement|DisableMovement _charactermovement)
      (if (> (Variables|Default|GetHealth) 0.1)
        ;;[1 1 1] Still Alive
        (Components|Animation|PlayAnimation (Variables|Character|GetMesh) "/Game/Guy/Character_AlienEnemy/Animations/Head_Hit.Head_Hit" false)
        (Utilities|FlowControl|Delay 1.3)
        (Variables|Default|SetGetDamage? false)
        (Components|Animation|SetAnimationMode (Variables|Character|GetMesh) "AnimationBlueprint") ; ?Returning the AnimBP
        (Pawn|Components|CharacterMovement|SetMovementMode (Variables|Character|GetCharacterMovement) "MOVE_Walking" 0)
        (else
          ;;[1 1 1] Death
          (Variables|Default|SetDead? true)
          (Collision|SetCollisionEnabled (Variables|Collision|GetCapsuleComponent) "NoCollision")
          (Utilities|FlowControl|Delay 0.4)
          (if (Utilities|Enum|Equal(Enum) (Class|SkeletalMeshComponent|GetAnimationMode (Variables|Character|GetMesh)) "AnimationSingleNode")
            (Utilities|FlowControl|Delay 1.0) ; In case of mix between animations - playing default death animation after a bigger delay\n* Dont delete * - Without it the Idle animation can be stuck instead of deathing
            (Components|Animation|PlayAnimation (Variables|Character|GetMesh) "/Game/Guy/Character_AlienEnemy/Animations/Death_From_Back_Headshot.Death_From_Back_Headshot" false :!label _label)
            (else
              (switch int (Math|Random|RandomIntegerinRange 0 3)
                (:Default
                  (goto _label))
                (:0
                  (goto _label))
                (:1
                  (Components|Animation|PlayAnimation (Variables|Character|GetMesh) "/Game/Guy/Character_AlienEnemy/Animations/Death_From_Front_Headshot.Death_From_Front_Headshot" false))
                (:2
                  (Components|Animation|PlayAnimation (Variables|Character|GetMesh) "/Game/Guy/Character_AlienEnemy/Animations/Falling_Back_Death.Falling_Back_Death" false))
                (:3
                  (Components|Animation|PlayAnimation (Variables|Character|GetMesh) "/Game/Guy/Character_AlienEnemy/Animations/Falling_Forward_Death.Falling_Forward_Death" false)))))
          (Utilities|FlowControl|Delay 12.0)
          (Actor|DestroyActor))))))

(event OnSeePawn(PawnSensing(Eyes))
  (params (Pawn :type Pawn%20Object%20Reference))
  (bind _mesh (Variables|Character|GetMesh))
  ;[1 1 1] AI Chase Player & Sound
  ;;[1 1 1] Eyes - Chase Player
  ;;;[0 1 0.1918] On See Pawn
  (if (not (Variables|Default|GetDead?))
    (Utilities|FlowControl|Sequence
      (:then_0
        ;;;[1 1 1] Chase Runner
        (bind _ascharacter_runner_bp_side_knifes (Utilities|Casting|CastToCharacter_RunnerBP_SideKnifes Pawn)) ; Runner
        (Utilities|FlowControl|Sequence
          (:then_0
            (Variables|Default|SetCanSee? true)
            (Variables|/Script/Engine.CharacterMovementComponent|SetMaxWalkSpeed (Variables|Character|GetCharacterMovement) (Variables|Default|GetMAX_RUN))
            (AI|AIMoveTo self "0, 0, 0" _ascharacter_runner_bp_side_knifes 5.0 false
              (:OnSuccess
                ;;;;[0.84 0.05074 0] Attack Runner
                ;;;;;[0 0.5639 1] Zombie Actions
                (Utilities|FlowControl|Delay 0.3)
                (if (not (Variables|Default|GetGetDamage?)) ; Disable attack when getting damage
                  (if (not (Variables|Default|GetDead?)) ; Disable attack when dead
                    (bind _ascharacter_runner_bp_side_knifes_2 (Utilities|Casting|CastToCharacter_RunnerBP_SideKnifes (Game|GetPlayerCharacter 0)))
                    (if (not (Variables|/Game/Guy/Blueprints/Character_RunnerBP_SideKnifes.Character_RunnerBP_SideKnifes_C|GetDead? _ascharacter_runner_bp_side_knifes_2))
                      (Components|Animation|PlayAnimation _mesh "/Game/Guy/Character_AlienEnemy/Animations/Bash.Bash" false) ; Zombie animation
                      (Utilities|FlowControl|Delay 1.0)
                      (Components|Animation|SetAnimationMode _mesh "AnimationBlueprint")
                      (if (Variables|Default|GetCanSee?)
                        ;;;;;[0 1 0.03957] Game Mode
                        (bind _asmaze_game_mode (Utilities|Casting|CastToMaze_GameMode (Game|GetGameMode)))
                        (if (Variables|/Game/Guy/Blueprints/Character_RunnerBP_SideKnifes.Character_RunnerBP_SideKnifes_C|GetBlocking? _ascharacter_runner_bp_side_knifes_2)
                          (Variables|/Game/Guy/Blueprints/Maze_GameMode.Maze_GameMode_C|SetHealth _asmaze_game_mode (- (Variables|/Game/Guy/Blueprints/Maze_GameMode.Maze_GameMode_C|GetHealth _asmaze_game_mode) (Variables|Default|GetBlockingPlayerTakeDamage)))
                          (else
                            (Variables|/Game/Guy/Blueprints/Maze_GameMode.Maze_GameMode_C|SetHealth _asmaze_game_mode (- (Variables|/Game/Guy/Blueprints/Maze_GameMode.Maze_GameMode_C|GetHealth _asmaze_game_mode) (Variables|Default|GetPlayerTakeDamage)))))
                        ;;;;;[1 1 1] Runner Actions
                        (Components|Movement|StopMovementImmediately (Variables|/Script/Engine.Character|GetCharacterMovement _ascharacter_runner_bp_side_knifes_2))
                        (Pawn|Components|CharacterMovement|DisableMovement (Variables|/Script/Engine.Character|GetCharacterMovement _ascharacter_runner_bp_side_knifes_2))
                        (if (> (Variables|/Game/Guy/Blueprints/Maze_GameMode.Maze_GameMode_C|GetHealth _asmaze_game_mode) 0.01)
                          ;;;;;;[1 1 1] Still Alive
                          (Components|Animation|PlayAnimation (Variables|/Script/Engine.Character|GetMesh _ascharacter_runner_bp_side_knifes_2) "/Game/Guy/Character_Runner/Animations/Head_Hit__1_.Head_Hit__1_" false)
                          (Utilities|FlowControl|Delay 1.3)
                          (Components|Animation|SetAnimationMode (Variables|/Script/Engine.Character|GetMesh _ascharacter_runner_bp_side_knifes_2) "AnimationBlueprint") ; ?Returning to the AnimBP
                          (Pawn|Components|CharacterMovement|SetMovementMode (Variables|/Script/Engine.Character|GetCharacterMovement _ascharacter_runner_bp_side_knifes_2) "MOVE_Walking" 0)
                          (else
                            ;;;;;;[1 1 1] Death
                            (Variables|/Game/Guy/Blueprints/Character_RunnerBP_SideKnifes.Character_RunnerBP_SideKnifes_C|SetDead? _ascharacter_runner_bp_side_knifes_2 true)
                            (Utilities|FlowControl|Delay 0.4)
                            (Components|Movement|StopMovementImmediately (Variables|/Script/Engine.Character|GetCharacterMovement _ascharacter_runner_bp_side_knifes_2))
                            (Pawn|Components|CharacterMovement|DisableMovement (Variables|/Script/Engine.Character|GetCharacterMovement _ascharacter_runner_bp_side_knifes_2))
                            (if (Utilities|Enum|Equal(Enum) (Class|SkeletalMeshComponent|GetAnimationMode (Variables|/Script/Engine.Character|GetMesh _ascharacter_runner_bp_side_knifes_2)) "AnimationSingleNode")
                              (Utilities|FlowControl|Delay 1.0) ; In case of mix between animations - playing default death animation after a bigger delay\n* Dont delete * - Without it the Idle animation can be stuck instead of deathing
                              (Components|Animation|PlayAnimation (Variables|/Script/Engine.Character|GetMesh _ascharacter_runner_bp_side_knifes_2) "/Game/Guy/Character_Runner/Animations/Dying__1_.Dying__1_" false :!label _label)
                              (else
                                (switch int (Math|Random|RandomIntegerinRange 0 3)
                                  (:Default
                                    (goto _label))
                                  (:0
                                    (goto _label))
                                  (:1
                                    (Components|Animation|PlayAnimation (Variables|/Script/Engine.Character|GetMesh _ascharacter_runner_bp_side_knifes_2) "/Game/Guy/Character_Runner/Animations/Dying__1_.Dying__1_" false))
                                  (:2
                                    (Components|Animation|PlayAnimation (Variables|/Script/Engine.Character|GetMesh _ascharacter_runner_bp_side_knifes_2) "/Game/Guy/Character_Runner/Animations/Dying__1_.Dying__1_" false))
                                  (:3
                                    (Components|Animation|PlayAnimation (Variables|/Script/Engine.Character|GetMesh _ascharacter_runner_bp_side_knifes_2) "/Game/Guy/Character_Runner/Animations/Dying__1_.Dying__1_" false)))))
                            ;;;;;;;[1 1 1] You Dead Message
                            (Utilities|FlowControl|Sequence
                              (:then_0
                                (Utilities|FlowControl|DoOnce false
                                  (:Completed
                                    (bind _returnvalue (UserInterface|CreateWidget "/Game/Guy/Blueprints/YouDead_Widget.YouDead_Widget_C" (Game|GetPlayerController 0)))
                                    (UserInterface|Viewport|AddtoViewport _returnvalue 0))))
                              (:then_1
                                (bind _asplayer_controller (Utilities|Casting|CastToPlayerController (Game|GetPlayerController 0)))
                                (Variables|/Script/Engine.PlayerController|SetbShowMouseCursor _asplayer_controller true))))))))))))
          (:then_1
            ;;;;[1 1 1] Hide eyes
            (Utilities|FlowControl|RetriggerableDelay 0.6)
            (Variables|/Script/Engine.CharacterMovementComponent|SetMaxWalkSpeed (Variables|Character|GetCharacterMovement) (Variables|Default|GetMAX_WALK))
            (Variables|Default|SetCanSee? false)))))))

(event EventBeginPlay
  ;[1 1 1] AI Chase Player & Sound
  ;;[1 1 1] Load Sound
)

(event Collision|EventActorBeginOverlap
  (params (OtherActor :type Actor%20Object%20Reference)))

(event EventTick
  (params (DeltaSeconds :type Float%20%28single-precision%29))
  (Utilities|FlowControl|Sequence
    (:then_0
      ;[1 1 1] Walk
      (if (not (Variables|Default|GetDead?))
        (if (not (Variables|Default|GetCanSee?))
          (if (not (Variables|Default|GetGetDamage?))
            (Utilities|FlowControl|Delay (Math|Random|RandomFloatinRange 1.0 5.0))
            (AI|AIMoveTo self (.RandomLocation (AI|Navigation|GetRandomReachablePointinRadius (Transformation|GetActorLocation) 1.5e+03 0 0)) 0 5.0 true)))))
    (:then_1
      ;[1 1 1] AI Chase Player & Sound
      ;;[1 1 1] Event Tick - Fade out sound
      (if (not (Variables|Default|GetCanSee?))
        (Utilities|FlowControl|Delay 0.4)
        (if (not (Variables|Default|GetCanSee?))
          ;;[1 1 1] Eyes - Chase Player
          ;;;[1 1 1] Chase Runner
          ;;;;[0 0.3557 1] Play Sound
          (Utilities|FlowControl|DoOnce false ; enters at Reset. Connect if want sound\nReset should be connected to fade out sound
            (:Completed
              (Audio|Components|Audio|Play 0.0))))))))

(fn ConstructionScript)